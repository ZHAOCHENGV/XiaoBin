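; Projectile actor for spell VFX that flies forward and plays configurable cast, projectile and impact effects.
; BeginPlay fires the cast and projectile effects, sets a local forward velocity, then retires the cast effect after short delays.
; A sphere hit on another actor stops movement, drives the projectile's Alpha parameter through a timeline and swaps to the impact effect at the hit location.
; If Destroy is set, delayed cleanup removes the actor.
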(event `self.ReceiveBeginPlay`
  (bind _cast (`self.Cast`))
  (`NiagaraComponent.SetAsset` (`self.Cast`) (`self.CastVFX`))
  (`ActorComponent.SetActive` (`self.Cast`) true false)
  (`ProjectileMovementComponent.SetVelocityInLocalSpace` (`self.ProjectileMovement`) (1500.0 0.0 0.0))
  (`self.SpawnProjectile`)
  (`KismetSystemLibrary.Delay` 1.0)
  (`ActorComponent.Deactivate` _cast)
  (`KismetSystemLibrary.Delay` 1.0)
  (`ActorComponent.K2_DestroyComponent` _cast))

(event `SpawnProjectile`
  (`NiagaraComponent.SetAsset` (`self.Projectile`) (`self.ProjectileVFX`))
  (`ActorComponent.SetActive` (`self.Projectile`) true false))

(event `self.Sphere_Collision.OnComponentHit`
  (params (HitComponent :type "PrimitiveComponent Object Reference") (OtherActor :type "Actor Object Reference") (OtherComp :type "PrimitiveComponent Object Reference") (NormalImpulse :type "Vector Structure") (Hit :type "HitResult Structure (by ref)"))
  (if (not (== OtherActor self))
    (`MovementComponent.StopMovementImmediately` (`self.ProjectileMovement`))
    (`|ExecutionSequence`
      (:`then_0`
        (bind (_direction _alpha) (`Timeline|AlphaTime` :!via `PlayFromStart`)
          (:`Update`
            (`FXSystemComponent.SetFloatParameter` (`self.Projectile`) "Alpha" _alpha))))
      (:`then_1`
        (`ActorComponent.Deactivate` (`self.Projectile`))
        (`NiagaraComponent.SetAsset` (`self.Impact`) (`self.ImpactVFX`))
        (`SceneComponent.K2_SetWorldLocation` (`self.Impact`) (`.Location` (`GameplayStatics.BreakHitResult` Hit)) false false)
        (`ActorComponent.SetActive` (`self.Impact`) true false)
        (if (`self.Destroy?`)
          (`KismetSystemLibrary.Delay` 1.0)
          (`ActorComponent.K2_DestroyComponent` (`self.Projectile`))
          (`KismetSystemLibrary.Delay` 1.0)
          (`self.K2_DestroyActor`))))))

(fn `UserConstructionScript`)