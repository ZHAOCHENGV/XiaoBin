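; BP_Water is a stylized water actor that sets up a scalable ocean surface with caustics and an underwater look.
; The construction script assigns materials to the surface, underwater plane and caustics decal, applies the ocean scale, and configures post-process settings with the underwater material and blend values.
; On actor overlap, it writes the water plane's doubled world location into MPC_Water as "Water Height" for materials to read.
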(event `self.ReceiveActorBeginOverlap`
  (params (OtherActor :type "Actor Object Reference"))
  (`KismetMaterialLibrary.SetVectorParameterValue` "/Game/WaterStylizedCustom/Material/MaterialParameter/MPC_Water.MPC_Water" "Water Height" (`KismetMathLibrary.Conv_VectorToLinearColor` (* (`SceneComponent.K2_GetComponentLocation` (`self.WaterPlane`)) 2.0))))

(fn `UserConstructionScript`
  (bind _oceanscale (`self.OceanScale`))
  (`PrimitiveComponent.SetMaterial` (`self.UnderWaterPlane`) 0 (`self.Underwater Material`))
  (`PrimitiveComponent.SetMaterial` (`self.WaterPlane`) 0 (`self.WaterMaterial`))
  (`DecalComponent.SetDecalMaterial` (`self.Decal`) (`self.CausticsDecalMaterial`))
  (`self.SetActorScale3D` _oceanscale)
  (`SceneComponent.SetWorldScale3D` (`self.Decal`) _oceanscale)
  (bind _output_get (set `self.PostProcess` (`self.PostProcess`)))
  (set `PostProcessComponent.Settings` (make `PostProcessSettings` :`ColorGain` (`self.Gain`) :`SceneColorTint` (struct :`R` 0.428691 :`G` 0.428691 :`B` 0.428691 :`A` 1.0) :`SceneFringeIntensity` 0.8 :`BloomIntensity` 2.0 :`BloomDirtMask` "/Game/WaterStylizedCustom/Tex/T_ScreenDirt_BC.T_ScreenDirt_BC" :`BloomDirtMaskIntensity` 8.0 :`AutoExposureLowPercent` 80.0 :`AutoExposureHighPercent` 93.0 :`AutoExposureMinBrightness` 0.05 :`AutoExposureMaxBrightness` 2.0 :`AutoExposureSpeedUp` 5.0 :`AutoExposureSpeedDown` 5.0 :`VignetteIntensity` 0.8 :`AmbientOcclusionIntensity` 1.0 :`DepthOfFieldFocalRegion` 2000.0 :`DepthOfFieldFarTransitionRegion` 2000.0 :`MotionBlurAmount` 1.0 :`WeightedBlendables` (`self.UnderwaterMaterial`) :`LPVSize` 2000.0 :`LPVSecondaryOcclusionIntensity` 1.0 :`LPVDirectionalOcclusionIntensity` 0.3 :`LPVDirectionalOcclusionRadius` 6.0) _output_get)
  (set `PostProcessComponent.BlendRadius` (`self.UnderwaterBlendRadius`) _output_get)
  (set `PostProcessComponent.BlendWeight` (`self.UnderwaterBlendWeight`) _output_get))