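; BP_ConfigCameraPawn is a configuration camera pawn Blueprint that shows and hides the placement (create) menu.
; On BeginPlay it binds to three delegates: show menu, hide menu and config confirmed.
; A show request creates a new WBP_CreateMenu, stores it and adds it to the viewport.
; A hide request or config confirmation removes the stored widget from its parent.
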(event `self.ReceiveBeginPlay`
  (add `self.OnRequestShowPlacementMenu` (delegate `OnRequestShowPlacementMenu_事件`))
  (add `self.OnRequestHidePlacementMenu` (delegate `OnRequestHidePlacementMenu_事件`))
  (add `self.OnConfigConfirmed` (delegate `OnConfigConfirmed_事件`)))

(event `OnRequestShowPlacementMenu_事件`
  (bind _returnvalue (`|CreateWidget` "/Game/UI/WBP_CreateMenu.WBP_CreateMenu_C"))
  (bind _output_get (set `self.创造菜单` _returnvalue))
  (`UserWidget.AddToViewport` _returnvalue 0)
  (`UserWidget.AddToViewport` _output_get 0))

(event `OnRequestHidePlacementMenu_事件`
  (`Widget.RemoveFromParent` (`self.创造菜单`)))

(event `OnConfigConfirmed_事件`
  (`Widget.RemoveFromParent` (`self.创造菜单`)))

(fn `UserConstructionScript`)